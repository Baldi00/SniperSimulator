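; BP_SniperPlayer is the sniper simulator's player Blueprint, which here handles 2D sound feedback for shooting and related actions.
; BeginPlay caches the SniperSimulatorGameState, whose killcam and silencer flags select the bullet-time, silenced or standard shot sound.
; Separate events play the long-distance hit, click and breath sounds.
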(event EventPlayShootSound
  (bind _gamestate (Variables|Default|GetGameState))
  (if (Variables|/Script/SniperSimulator.SniperSimulatorGameState|GetbUseKillcam _gamestate)
    (Audio|PlaySound2D "/Game/SniperSimulator/Art/Sounds/SFX_Shoot_Bullet_Time.SFX_Shoot_Bullet_Time" 1.0 1.0 0.0 0 0)
    (elif (Variables|/Script/SniperSimulator.SniperSimulatorGameState|GetbShootSilenced _gamestate)
      (Audio|PlaySound2D "/Game/SniperSimulator/Art/Sounds/SFX_Shoot_Silenced.SFX_Shoot_Silenced" 1.0 1.0 0.0 0 0)
      (else
        (Audio|PlaySound2D "/Game/SniperSimulator/Art/Sounds/SFX_Shoot.SFX_Shoot" 1.0 1.0 0.0 0 0)))))

(event EventPlayFarHitSound
  (Audio|PlaySound2D "/Game/SniperSimulator/Art/Sounds/SFX_Shot_Long_Distance_Hit.SFX_Shot_Long_Distance_Hit" 1.0 1.0 0.0 0 0))

(event EventBeginPlay
  (bind _assniper_simulator_game_state (Utilities|Casting|CastToSniperSimulatorGameState (Game|GetGameState)))
  (Variables|Default|SetGameState _assniper_simulator_game_state))

(event EventPlayClickSound
  (Audio|PlaySound2D "/Engine/VREditor/Sounds/UI/Flashlight_Switch.Flashlight_Switch" 1.0 1.0 0.0 0 0))

(event EventPlayBreathSound
  (Audio|PlaySound2D "/Game/SniperSimulator/Art/Sounds/SFX_Breath.SFX_Breath" 1.0 1.0 0.0 0 0))

(fn ConstructionScript)