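; BP_Robot is a robot target for the sniper simulator that collapses into a ragdoll when a bullet hits it.
; On its first BulletHit, the skeletal mesh switches to the Ragdoll collision profile, starts simulating physics and receives a large force along the bullet direction.
; Killcam hits also play a 2D hit sound.
; An AlreadyHit flag blocks repeat reactions and is exposed through IsAlreadyHit.
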(event EventBulletHit
  (params (InDirection :type Vector :default "0, 0, 0") (bInIsKillcam :type Boolean))
  (bind _skeletalmesh (Variables|Default|GetSkeletalMesh))
  (if (not (Variables|Default|GetbAlreadyHit))
    (Variables|Default|SetbAlreadyHit true)
    (Utilities|FlowControl|Sequence
      (:then_0
        (Collision|SetCollisionProfileName _skeletalmesh "Ragdoll" true :!class /Script/Engine.PrimitiveComponent)
        (Physics|SetSimulatePhysics _skeletalmesh true)
        (Physics|AddForce _skeletalmesh (* InDirection 3e+07) "None" false))
      (:then_1
        (if bInIsKillcam
          (Audio|PlaySound2D "/Game/SniperSimulator/Art/Sounds/SFX_Robot_Hit.SFX_Robot_Hit" 1.0 1.0 0.0 0 0))))))

(fn ConstructionScript)

(fn IsAlreadyHit
  (return (Variables|Default|GetbAlreadyHit)))