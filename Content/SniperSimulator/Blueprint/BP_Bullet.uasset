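; BP_Bullet is the sniper bullet actor that carries its own follow camera on a spring arm.
; While animating, Tick sways the spring arm socket with real-time sine and cosine waves and keeps the camera looking at the bullet mesh.
; HideMeshandStopCamera hides the mesh and ends the animation, after which Tick eases the socket offset, arm length and camera rotation to a fixed resting view.
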(event EventTick
  (params (DeltaSeconds :type Float%20%28single-precision%29))
  (bind _returnvalue (Utilities|Time|GetRealTimeSeconds))
  (bind _camera (Variables|Default|GetCamera))
  (bind _camera_2 (Variables|Default|GetCamera))
  (bind _springarm (Variables|Default|GetSpringArm))
  (if (Variables|Default|GetbIsAnimatingCamera)
    (Variables|/Script/Engine.SpringArmComponent|SetSocketOffset (Variables|Default|GetSpringArm) (Math|Vector|MakeVector (* (Math|Trig|Cos(Radians) (* _returnvalue 1.6)) 2e+01) (* (Math|Trig|Sin(Radians) (* _returnvalue 1.0)) 5e+01) (* (Math|Trig|Sin(Radians) (* _returnvalue 1.25)) 5.0)))
    (Transformation|SetWorldRotation _camera (Math|Rotator|FindLookatRotation (Transformation|GetWorldLocation _camera) (Transformation|GetWorldLocation (Variables|Default|GetBulletMesh))) false false)
    (else
      (Variables|/Script/Engine.SpringArmComponent|SetSocketOffset (Variables|Default|GetSpringArm) (Math|Interpolation|VInterpTo (Variables|/Script/Engine.SpringArmComponent|GetSocketOffset (Variables|Default|GetSpringArm)) "10.000000,0.000000,10.000000" DeltaSeconds 5.0))
      (Variables|/Script/Engine.SpringArmComponent|SetTargetArmLength _springarm (Math|Interpolation|FInterpTo (Variables|/Script/Engine.SpringArmComponent|GetTargetArmLength _springarm) 5e+02 DeltaSeconds 5.0))
      (Transformation|SetRelativeRotation _camera_2 (Math|Interpolation|RInterpTo (Variables|/Script/Engine.SceneComponent|GetRelativeRotation _camera_2) "0, 0, 0" DeltaSeconds 5.0) false false))))

(event EventHideMeshandStopCamera
  (Variables|Default|SetbIsAnimatingCamera false)
  (Rendering|SetVisibility (Variables|Default|GetBulletMesh) false false))

(fn ConstructionScript)