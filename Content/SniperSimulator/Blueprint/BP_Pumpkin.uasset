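; BP_Pumpkin is a shootable pumpkin target in the sniper simulator, built around a Geometry Collection.
; Its BulletHit event acts only once, latched by an AlreadyHit flag that IsAlreadyHit exposes.
; On that hit it spawns a scaled-up, one-second BP_ForceField at the Geometry Collection's location, and plays a bullet impact sound if the shot is a killcam.
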(event EventBulletHit
  (params (InDirection :type Vector :default "0, 0, 0") (bInIsKillcam :type Boolean))
  (if (not (Variables|Default|GetbAlreadyHit))
    (Variables|Default|SetbAlreadyHit true)
    (Utilities|FlowControl|Sequence
      (:then_0
        (if bInIsKillcam
          (Audio|PlaySound2D "/Game/SniperSimulator/Art/Sounds/SFX_Bullet_Enter_Body.SFX_Bullet_Enter_Body" 1.0 1.0 0.0 0 0)))
      (:then_1
        (bind _returnvalue (Game|SpawnActorfromClass "/Game/SniperSimulator/Blueprint/BP_ForceField.BP_ForceField_C" (Math|Transform|MakeTransform (Transformation|GetWorldLocation (Variables|Default|GetGeometryCollection)) "0, 0, 0" "2.000000,2.000000,2.000000") "Undefined" "MultiplyWithRoot" 0 0))
        (Actor|SetLifeSpan _returnvalue 1.0)))))

(fn ConstructionScript)

(fn IsAlreadyHit
  (return (Variables|Default|GetbAlreadyHit)))